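; Healing pickup that restores the player to maximum health once on overlap with its hit box, then destroys itself.
; Construction randomly picks one of two Langos materials and stores a dynamic instance showing half the texture width.
; On pickup, it calls the character's heal and plays a sound, then Die waits briefly, plays a crush sound and shifts the texture's X offset as a two-frame death animation before removing the actor.
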(event `self.HitBox.OnComponentBeginOverlap`
  (params (OverlappedComponent :type "PrimitiveComponent Object Reference") (OtherActor :type "Actor Object Reference") (OtherComp :type "PrimitiveComponent Object Reference") (OtherBodyIndex :type Integer) (bFromSweep :type Boolean) (SweepResult :type "HitResult Structure (by ref)"))
  ;[1 1 1] Heal player
  (if (and (`self.IsAlive`) (== OtherActor (`GameplayStatics.GetPlayerPawn` 0)))
    (set `self.IsAlive` false)
    (`/Engine/EditorBlueprintResources/StandardMacros.IsValid` OtherActor
      (:`Is Valid`
        (if true
          (bind _asbp_first_person_character (cast `/Game/FirstPerson/Blueprints/BP_FirstPersonCharacter` OtherActor))
          (`/Game/FirstPerson/Blueprints/BP_FirstPersonCharacter.HealToMaximum` _asbp_first_person_character)
          (`GameplayStatics.PlaySound2D` "/Game/Sounds/Effects/GETITM19.GETITM19" 1.0 1.0 0.0 null null)
          (`self.Die`))))))

(fn `UserConstructionScript`
  (bind _staticmesh (`self.StaticMesh`))
  ;[1 1 1] Set random material for static mesh
  (bind _output_get (set `self.IsType1` (`KismetMathLibrary.RandomBool`)))
  (if _output_get
    (bind _returnvalue (`PrimitiveComponent.CreateDynamicMaterialInstance` _staticmesh 0 "/Game/Obstacles/Assets/M_Langos_1.M_Langos_1" "Langos_1"))
    (`MaterialInstanceDynamic.SetScalarParameterValue` _returnvalue "TilingX" 0.5)
    (set `self.MaterialRef` _returnvalue)
    (else
      (bind _returnvalue_2 (`PrimitiveComponent.CreateDynamicMaterialInstance` _staticmesh 0 "/Game/Obstacles/Assets/M_Langos_2.M_Langos_2" "Langos_2"))
      (`MaterialInstanceDynamic.SetScalarParameterValue` _returnvalue_2 "TilingX" 0.5)
      (set `self.MaterialRef` _returnvalue_2))))